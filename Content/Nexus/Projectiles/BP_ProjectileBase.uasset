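; Base projectile actor that reports its impact to the Gameplay Ability System and then destroys itself.
; The construction script binds the collision sphere's hit event to a handler that sends a tagged gameplay event to the Instigator, with Damage as magnitude and the hit result as target data.
; The handler also spawns a scaled-up impact emitter at the hit point, and applies no damage itself.
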(fn ConstructionScript
  (Collision|BindEventtoOnComponentHit (Variables|Default|GetCollisionSphere) (EventDispatchers|CreateEvent :!event BPProjectileBaseAutoGenFunc)))

(fn BPProjectileBaseAutoGenFunc
  (params (HitComponent :type Primitive%20Component%20Object%20Reference) (OtherActor :type Actor%20Object%20Reference) (OtherComp :type Primitive%20Component%20Object%20Reference) (NormalImpulse :type Vector) (Hit :type Hit%20Result%20Structure%20%28by%20ref%29))
  (bind _instigator (Variables|Default|GetInstigator))
  (Ability|SendGameplayEventtoActor _instigator (Variables|ProjectileSettings|GetEvent%20Tag) (Utilities|Struct|MakeGameplayEventData "(TagName=\"\")" _instigator 0 0 0 "()" "(GameplayTags=)" "(GameplayTags=)" (Variables|Default|GetDamage) (Ability|TargetData|AbilityTargetDatafromHitResult Hit)))
  (Effects|SpawnEmitteratLocation (Variables|ProjectileSettings|GetEmitter%20Template) (.ImpactPoint (Collision|BreakHitResult Hit)) "0, 0, 0" "5.000000,5.000000,5.000000")
  (Actor|DestroyActor)
  (return))
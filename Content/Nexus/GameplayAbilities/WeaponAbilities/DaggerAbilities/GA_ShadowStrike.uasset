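; Shadow Strike gameplay ability for daggers, activated by a gameplay event, that runs a melee hitscan on the instigator's equipped weapon.
; Activation commits the cost, while the cooldown is committed when the ability ends.
; On authority only, one-shot waits for the HitScan Start and End events open and close the weapon's hitscan, with damage taken from the event magnitude.
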(event Ability|EventOnEndAbility
  (params (bWasCancelled :type Boolean))
  (Ability|CommitAbilityCooldown false))

(event Ability|EventActivateAbilityFromEvent
  (params (EventData :type Gameplay%20Event%20Data%20Structure%20%28by%20ref%29))
  (bind (_eventtag _instigator _target _optionalobject _optionalobject2 _contexthandle _instigatortags _targettags _eventmagnitude) (Utilities|Struct|BreakGameplayEventData EventData))
  (Ability|CommitAbilityCost false)
  (Variables|Default|SetAs%20BP%20Weapon%20Melee%20Base (.AsNexus%20Melee%20Weapon%20Base (Utilities|Casting|CastToNexusMeleeWeaponBase (Variables|/Script/Nexus.NexusWeaponsManager|GetEquippedWeapon (Variables|/Script/Nexus.NexusPlayerCharacter|GetWeaponsManager (.AsNexus%20Player%20Character (Utilities|Casting|CastToNexusPlayerCharacter _instigator)))))))
  (Ability|HasAuthority
    (:True
      (Ability|Tasks|WaitGameplayEvent "(TagName=\"Event.HitScan.Start\")" 0 true
        (:then
          (Ability|Tasks|WaitGameplayEvent "(TagName=\"Event.HitScan.End\")" 0 true
            (:EventReceived
              (Class|NexusMeleeWeaponBase|EndHitscan (Variables|Default|GetAs%20BP%20Weapon%20Melee%20Base)))))
        (:EventReceived
          (Variables|/Script/Nexus.NexusMeleeWeaponBase|SetDamageToDeal (Variables|Default|GetAs%20BP%20Weapon%20Melee%20Base) _eventmagnitude)
          (Class|NexusMeleeWeaponBase|StartHitscan (Variables|Default|GetAs%20BP%20Weapon%20Melee%20Base)))))))
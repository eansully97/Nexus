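; Event-triggered gameplay ability that deals area damage when a projectile explodes.
; It sphere-traces for Pawns at the event's impact point within EffectRadius and collects unique hit actors.
; Actors on another team without Status.Block receive GE_Damage_Default, with the event magnitude passed as SetByCaller Data.Damage.
; Each target's own ASC builds and applies the spec, and a same-team hit calls EndAbility inside the loop.
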(event Ability|EventActivateAbility)

(event Ability|EventOnEndAbility
  (params (bWasCancelled :type Boolean)))

(event Ability|EventActivateAbilityFromEvent
  (params (EventData :type Gameplay%20Event%20Data%20Structure%20%28by%20ref%29))
  (bind (_eventtag _instigator _target _optionalobject _optionalobject2 _contexthandle _instigatortags _targettags _eventmagnitude _targetdata) (Utilities|Struct|BreakGameplayEventData EventData))
  (bind _hitactors (Variables|Default|GetHitActors))
  (bind _returnvalue (Ability|TargetData|GetHitResultfromTargetData _targetdata))
  (bind _impactpoint (Collision|BreakHitResult _returnvalue))
  (Utilities|Array|Clear (Variables|Default|GetHitActors))
  (bind (_outhits _returnvalue_2) (Collision|MultiSphereTraceForObjects _impactpoint _impactpoint (Variables|Default|GetEffectRadius) (Utilities|Array|MakeArray "ObjectTypeQuery3") false 0 "None"))
  (if _returnvalue_2
    (for _array_element _outhits
      (Utilities|IsValid (.HitActor (Collision|BreakHitResult _array_element))
        (:Is%20Valid
          (Variables|Default|SetHit%20Actor (.HitActor (Collision|BreakHitResult _array_element)))
          (if (not (Utilities|Array|ContainsItem (Variables|Default|GetHitActors) (Variables|Default|GetHit%20Actor)))
            (Utilities|Array|AddUnique (Variables|Default|GetHitActors) (Variables|Default|GetHit%20Actor))))
        (:Is%20Not%20Valid
          (Ability|EndAbility))))
    (if (Utilities|Array|IsNotEmpty _hitactors)
      (for _array_element_2 _hitactors
        (Variables|Default|SetActorToDamage _array_element_2)
        (if (Utilities|Enum|Equal(Enum) (Class|NexusCharacterBase|GetTeamID (.AsNexus%20Character%20Base (Utilities|Casting|CastToNexusCharacterBase (Ability|GetAvatarActorfromActorInfo)))) (Class|NexusCharacterBase|GetTeamID (.AsNexus%20Character%20Base (Utilities|Casting|CastToNexusCharacterBase (Variables|Default|GetActorToDamage)))))
          (Ability|EndAbility)
          (elif (not (GameplayTags|HasMatchingGameplayTag (Ability|GetAbilitySystemComponent (.AsNexus%20Character%20Base (Utilities|Casting|CastToNexusCharacterBase (Variables|Default|GetActorToDamage)))) "(TagName=\"Status.Block\")"))
            (bind _returnvalue_3 (Ability|GameplayEffect|AssignTagSetbyCallerMagnitude (GameplayEffects|MakeOutgoingSpec (Ability|GetAbilitySystemComponent (.AsNexus%20Character%20Base (Utilities|Casting|CastToNexusCharacterBase (Variables|Default|GetActorToDamage)))) "/Game/Nexus/GameplayEffects/GE_Damage_Default.GE_Damage_Default_C" 0.0 (GameplayEffects|MakeEffectContext (Ability|GetAbilitySystemComponent (.AsNexus%20Character%20Base (Utilities|Casting|CastToNexusCharacterBase (Variables|Default|GetActorToDamage)))))) "(TagName=\"Data.Damage\")" _eventmagnitude))
            (GameplayEffects|ApplyGameplayEffectSpecToSelf (Ability|GetAbilitySystemComponent (.AsNexus%20Character%20Base (Utilities|Casting|CastToNexusCharacterBase (Variables|Default|GetActorToDamage)))) _returnvalue_3)))))
    (Ability|EndAbility)
    (else
      (Ability|EndAbility))))
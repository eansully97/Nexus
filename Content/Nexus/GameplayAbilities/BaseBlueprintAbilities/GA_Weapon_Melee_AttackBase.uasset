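; Base melee attack gameplay ability that plays an attack montage using the avatar's equipped Nexus melee weapon, ending if none is found.
; On the authority, hit-scan start and end gameplay events toggle the weapon's hitscan, passing in damage and radius at start.
; The ability ends when the montage completes, is interrupted or is cancelled, and ending always stops any hitscan on the cached weapon.
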(event Ability|EventActivateAbility
  (bind _returnvalue (Ability|GetAvatarActorfromActorInfo))
  (bind _returnvalue_2 (Actor|GetComponentbyClass _returnvalue "/Script/Nexus.NexusWeaponsManager"))
  (Ability|CommitAbility)
  (Utilities|IsValid _returnvalue_2
    (:Is%20Valid
      (bind _equippedweapon (Variables|/Script/Nexus.NexusWeaponsManager|GetEquippedWeapon _returnvalue_2)
        (:then
          (bind _asnexus_melee_weapon_base (Utilities|Casting|CastToNexusMeleeWeaponBase _equippedweapon)
            (:then
              (Variables|Default|SetEquipped%20Weapon _asnexus_melee_weapon_base)
              (|PlayMontageandWaitProxy "None" (Variables|Default|GetMontage%20to%20Play) (Variables|Default|GetRate) "None" true 1.0 0.0 true
                (:then
                  (Ability|HasAuthority
                    (:True
                      (Ability|Tasks|WaitGameplayEvent "(TagName=\"Event.HitScan.Start\")" 0
                        (:then
                          (Ability|Tasks|WaitGameplayEvent "(TagName=\"Event.HitScan.End\")" 0
                            (:EventReceived
                              (Class|NexusMeleeWeaponBase|EndHitscan (Variables|Default|GetEquipped%20Weapon)))))
                        (:EventReceived
                          (Variables|/Script/Nexus.NexusMeleeWeaponBase|SetDamageToDeal (Variables|Default|GetEquipped%20Weapon) (Variables|Default|GetDamage%20To%20Deal))
                          (Variables|/Script/Nexus.NexusMeleeWeaponBase|SetDamageHitScanRadius (Variables|Default|GetEquipped%20Weapon) (Variables|Default|GetDamage%20Hit%20Scan%20Radius))
                          (Class|NexusMeleeWeaponBase|StartHitscan (Variables|Default|GetEquipped%20Weapon)))))))
                (:OnCompleted
                  (Ability|EndAbility :!label _label))
                (:OnInterrupted
                  (goto _label))
                (:OnCancelled
                  (goto _label))))
            (:CastFailed
              (Ability|EndAbility))))
        (:else
          (Ability|EndAbility :!label _label_2))))
    (:Is%20Not%20Valid
      (goto _label_2))))

(event Ability|EventOnEndAbility
  (params (bWasCancelled :type Boolean))
  (bind _equipped_weapon (Variables|Default|GetEquipped%20Weapon)
    (:then
      (Class|NexusMeleeWeaponBase|EndHitscan _equipped_weapon))
    (:else)))
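; Gameplay ability that gives a Nexus character a short dash along its last movement input, or along actor forward when there is no input.
; Activation applies a set-by-caller cost and a constant root motion force, with exit velocity clamped to the movement component's max speed.
; A dash gameplay cue lasts until the ability ends when the force finishes, and the cooldown is applied on end rather than on activation.
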(event Ability|EventActivateAbility
  (bind _returnvalue (Ability|GetAvatarActorfromActorInfo))
  (bind _asnexus_character_base (Utilities|Casting|CastToNexusCharacterBase _returnvalue))
  (Class|NexusGameplayAbility|ApplyCostSetbyCaller -1.0)
  (Ability|Tasks|ApplyRootMotionConstantForce "None" (Math|Vector|SelectVector (Transformation|GetActorForwardVector _returnvalue) (Pawn|Components|PawnMovement|GetLastInputVector (Variables|/Script/Engine.Character|GetCharacterMovement _asnexus_character_base)) (Utilities|Operators|EqualEqual :A (Pawn|Components|PawnMovement|GetLastInputVector (Variables|/Script/Engine.Character|GetCharacterMovement _asnexus_character_base)))) 2e+03 0.3 false 0 "ClampVelocity" "0, 0, 0" (CallFunction|GetMaxSpeed)
    (:then
      (GameplayCue|AddGameplayCue :GameplayCueTag "(TagName=\"GameplayCue.Ability.Dash.Activate\")"))
    (:OnFinish
      (Ability|EndAbility))))

(event Ability|EventOnEndAbility
  (params (bWasCancelled :type Boolean))
  (Class|NexusGameplayAbility|ApplyCooldownSetbyCaller -1.0))

(fn GetMaxSpeed
  (bind _aspawn (Utilities|Casting|CastToPawn (Ability|GetAvatarActorfromActorInfo))
    (:then
      (if (Math|Float|NearlyEqual(Float) (Class|MovementComponent|GetMaxSpeed (Pawn|GetMovementComponent _aspawn)) 0.0 1e-06)
        _
        (else
          (return (Class|MovementComponent|GetMaxSpeed (Pawn|GetMovementComponent _aspawn))))))
    (:CastFailed
      _))
  (return 0.0))
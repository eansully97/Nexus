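; GA_Parry is an event-activated gameplay ability that plays the player parry montage and repels nearby enemies.
; As the montage starts, a sphere overlap around the avatar gathers characters from other teams.
; Each gets a velocity impulse backward along its own facing with slight lift, plus default damage through a SetByCaller effect spec.
; The ability ends when the montage completes, is interrupted or is cancelled.
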(event Ability|EventOnEndAbility
  (params (bWasCancelled :type Boolean)))

(event Ability|EventActivateAbilityFromEvent
  (params (EventData :type Gameplay%20Event%20Data%20Structure%20%28by%20ref%29))
  (bind _asnexus_character_base (Utilities|Casting|CastToNexusCharacterBase (Ability|GetAvatarActorfromActorInfo)))
  (bind _output_get (Variables|Default|SetAs%20Nexus%20Character%20Base _asnexus_character_base))
  (Variables|Default|SetInstigatorTeamID (Class|NexusCharacterBase|GetTeamID _output_get))
  (|PlayMontageandWaitProxy "None" "/Game/Nexus/Characters/PlayerCharacter/Animation/AM_Player_Parry.AM_Player_Parry" 1.0 "None" true 1.0 0.0 true
    (:then
      (bind _outactors (Collision|SphereOverlapActors (Transformation|GetActorLocation (Variables|Default|GetAs%20Nexus%20Character%20Base)) 7.5e+02 (Utilities|Array|MakeArray "ObjectTypeQuery3") 0 (Utilities|Array|MakeArray (Variables|Default|GetAs%20Nexus%20Character%20Base))))
      (for _array_element _outactors
        (bind _asnexus_character_base_2 (Utilities|Casting|CastToNexusCharacterBase _array_element))
        (bind _output_get_2 (Variables|Default|SetHitCharacter _asnexus_character_base_2))
        (if (not (Utilities|Enum|Equal(Enum) (Class|NexusCharacterBase|GetTeamID _output_get_2) (Variables|Default|GetInstigatorTeamID)))
          (Utilities|Array|AddUnique (Variables|Default|GetActorsToEffect) (Variables|Default|GetHitCharacter))))
      (for _array_element_2 (Variables|Default|GetActorsToEffect)
        (Utilities|IsValid _array_element_2
          (:Is%20Valid
            (Physics|AddImpulse (Variables|/Script/Engine.Character|GetCharacterMovement _array_element_2) (+ (* (Transformation|GetActorForwardVector _array_element_2) -1e+03) "0.000000,0.000000,100.000000") true)
            (bind _returnvalue (Ability|GameplayEffect|AssignTagSetbyCallerMagnitude (Ability|MakeOutgoingGameplayEffectSpec "/Game/Nexus/GameplayEffects/GE_Damage_Default.GE_Damage_Default_C") "(TagName=\"Data.Damage\")" -4e+01))
            (GameplayEffects|ApplyGameplayEffectSpecToSelf (Variables|/Script/Nexus.NexusCharacterBase|GetAbilitySystemComponent _array_element_2) _returnvalue)))))
    (:OnCompleted
      (Ability|EndAbility :!label _label))
    (:OnInterrupted
      (goto _label))
    (:OnCancelled
      (goto _label))))
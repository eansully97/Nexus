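; Axe block gameplay ability that puts the avatar in a blocking state for a limited time.
; On activation it commits cost, plays the block montage at reduced rate and adds a loose Status.Block tag.
; It ends after AbilityDuration or when the montage completes or is interrupted or cancelled.
; On end it applies a SetByCaller block cooldown effect, commits cooldown and removes the tag.
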(event Ability|EventActivateAbility
  (Ability|CommitAbilityCost false)
  (|PlayMontageandWaitProxy "None" "/Game/Nexus/Characters/PlayerCharacter/Animation/Axe/AM_Axe_Block.AM_Axe_Block" 0.1 "None" true 1.0 0.0 true
    (:then
      (bind _asnexus_character_base (Utilities|Casting|CastToNexusCharacterBase (Ability|GetAvatarActorfromActorInfo)))
      (bind _output_get (Variables|Default|SetAs%20BP%20Nexus%20Player _asnexus_character_base))
      (Ability|GameplayEffect|AddLooseGameplayTags _output_get (GameplayTags|MakeGameplayTagContainerfromTag "(TagName=\"Status.Block\")"))
      (Utilities|FlowControl|Delay (Variables|Default|GetAbilityDuration))
      (Ability|EndAbility))
    (:OnCompleted
      (Ability|EndAbility :!label _label))
    (:OnInterrupted
      (goto _label))
    (:OnCancelled
      (goto _label))))

(event Ability|EventOnEndAbility
  (params (bWasCancelled :type Boolean))
  (bind _returnvalue (Ability|GameplayEffect|AssignTagSetbyCallerMagnitude (Ability|MakeOutgoingGameplayEffectSpec "/Game/Nexus/GameplayEffects/Cooldowns/GE_BlockCooldown.GE_BlockCooldown_C") "(TagName=\"Data.Cooldown\")" (Variables|Default|GetCooldown)))
  (GameplayEffects|ApplyGameplayEffectSpecToSelf (Ability|GetAbilitySystemComponent (Ability|GetAvatarActorfromActorInfo)) _returnvalue)
  (Ability|CommitAbilityCooldown false)
  (Ability|GameplayEffect|RemoveLooseGameplayTags 0 (GameplayTags|MakeGameplayTagContainerfromTag "(TagName=\"Status.Block\")")))
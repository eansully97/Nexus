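; Minion enemy character Blueprint that manages its overhead widget and reaction to being stunned.
; After a short BeginPlay delay it binds and shows the widget, which hides on death.
; Async gameplay tag listeners on Status.Stunned play the stun montage and disable movement (add fires only once), then restore walking on removal.
; Helper graphs check blocking, validate living enemy targets and rotate an attacker toward its target.
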(event EventBeginPlay
  ;[1 0.0181 7.2e-05 0.5] BeginPlay
  (Utilities|FlowControl|Delay 0.2)
  (bind _aswbp_overhead_widget (Utilities|Casting|CastToWBP_OverheadWidget (UserInterface|GetWidget (Variables|Default|GetOverheadWidget))))
  (Class|NexusVitalsWidget|SetObservedPawn _aswbp_overhead_widget self)
  (Rendering|SetVisibility (Variables|Default|GetOverheadWidget) true false)
  (Ability|Tasks|WaitGameplayTagAddToActor 0 "(TagName=\"Status.Stunned\")" true
    (:then
      (Ability|Tasks|WaitGameplayTagRemoveFromActor 0 "(TagName=\"Status.Stunned\")"
        (:Removed
          (Animation|StopAnimMontage (Variables|Default|GetStunMontage))
          (Pawn|Components|CharacterMovement|SetMovementMode (Variables|Character|GetCharacterMovement) "MOVE_Walking" 0))))
    (:Added
      (Animation|PlayAnimMontage (Variables|Default|GetStunMontage) 1.0 "None")
      (Pawn|Components|CharacterMovement|SetMovementMode (Variables|Character|GetCharacterMovement) "MOVE_None" 0))))

(event EventOnDeathStarted
  (Rendering|SetVisibility (Variables|Default|GetOverheadWidget) false false))

(fn ConstructionScript
  (|CallParentFunction))